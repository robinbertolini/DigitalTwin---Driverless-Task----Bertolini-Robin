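; BP_Road is a road actor that builds its geometry along the Road spline in the construction script.
; Each pair of neighboring spline points gets a spline mesh component fitted to their local locations and tangents.
; A nested loop steps along the spline by SpaziaturaConi (cone spacing) but has an empty body.
; The static mesh placement meant for both sides, using LarghezzaStrada (road width), is disconnected; event graph logic is empty.
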(event EventBeginPlay)

(event Collision|EventActorBeginOverlap
  (params (OtherActor :type Actor%20Object%20Reference)))

(event EventTick
  (params (DeltaSeconds :type Float%20%28single-precision%29)))

(fn ConstructionScript
  (bind _road (Variables|Default|GetRoad))
  (for _index (range 0 (- (Spline|GetNumberOfSplinePoints (Variables|Default|GetRoad)) 2))
    (bind _returnvalue (AddComponent|AddSplineMeshComponent false))
    (SplineMesh|SetStartandEnd _returnvalue (.Location (Spline|GetLocationandTangentatSplinePoint _road _index "Local")) (.Tangent (Spline|GetLocationandTangentatSplinePoint _road _index "Local")) (.Location (Spline|GetLocationandTangentatSplinePoint _road (+ _index 1) "Local")) (.Tangent (Spline|GetLocationandTangentatSplinePoint _road (+ _index 1) "Local")) true :!class /Script/Engine.SplineMeshComponent)
    (for _index_2 (range 0 (Math|Float|Truncate (/ (Spline|GetSplineLength (Variables|Default|GetRoad)) (Variables|Default|GetSpaziaturaConi))))
      _)))